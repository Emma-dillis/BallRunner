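; BP_WinVolume is a level exit trigger that lets the game advance once all crystals are collected.
; On box overlap, it blocks with a printed message while any BP_Crystal_01 or BP_Crystal_02 actors remain; otherwise it fades the camera out and waits briefly.
; It then finds the current level name in a level-name array and opens the next entry, or only prints a message on the final level.
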(event `self.Box.OnComponentBeginOverlap`
  (params (OverlappedComponent :type "PrimitiveComponent Object Reference") (OtherActor :type "Actor Object Reference") (OtherComp :type "PrimitiveComponent Object Reference") (OtherBodyIndex :type Integer) (bFromSweep :type Boolean) (SweepResult :type "HitResult Structure (by ref)"))
  (bind _returnvalue (`self.Crystals`))
  (if _returnvalue
    (`KismetSystemLibrary.PrintString` "NIE ZEBRANO WSZYSTKICH KRYSZTAŁÓW")
    (else
      (`PlayerCameraManager.StartCameraFade` :`self` (`GameplayStatics.GetPlayerCameraManager` 0) :`ToAlpha` 1.0 :`Duration` 0.7 :`bHoldWhenFinished` true)
      (`KismetSystemLibrary.Delay` 3.0)
      (`self.Complete level`))))

(fn `Complete level`
  (bind _returnvalue (`self.Is_Final_level`))
  (if _returnvalue
    (`KismetSystemLibrary.PrintString` "TO JEST OSTATNI POZIOM")
    (else
      (`self.Load_Next_level`))))

(fn `Crystals`
  (returns (ReturnValue :type Boolean))
  (bind _outactors (`GameplayStatics.GetAllActorsOfClass` "/Game/blueprint/BP_Crystal_01.BP_Crystal_01_C"))
  (bind _outactors_2 (`GameplayStatics.GetAllActorsOfClass` "/Game/blueprint/BP_Crystal_02.BP_Crystal_02_C"))
  (return (or (> (`KismetArrayLibrary.Array_Length` _outactors_2) 0) (> (`KismetArrayLibrary.Array_Length` _outactors) 0))))

(fn `Get_Current_level_Index`
  (returns (ReturnValue :type Integer))
  (bind _returnvalue (`GameplayStatics.GetCurrentLevelName` true))
  (return (`KismetArrayLibrary.Array_Find` (`self.tab_LevelNames_01`) _returnvalue)))

(fn `Get_Next_level_name`
  (returns (Output :type String))
  (bind _returnvalue (`self.Get_Current_level_Index`))
  (return (`|GetArrayItem` (`self.tab_LevelNames_01`) (+ _returnvalue 1))))

(fn `Is_Final_level`
  (returns (ReturnValue :type Boolean))
  (bind _returnvalue (`self.Get_Current_level_Index`))
  (return (== _returnvalue (`KismetArrayLibrary.Array_LastIndex` (`self.tab_LevelNames_01`)))))

(fn `Load_Next_level`
  (bind _output (`self.Get_Next_level_name`))
  (`GameplayStatics.OpenLevel` (`KismetStringLibrary.Conv_StringToName` _output)))

(fn `UserConstructionScript`)